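; Main player character Blueprint that manages the local player's HUD in a networked game.
; The HUD widget is created for the locally controlled character, on BeginPlay for remote clients and on Possessed for the authority, covering both clients and listen-server host.
; DeathEvent removes the HUD from the screen.
; Keys 1-3 are test-only inputs copied from a UI test character that set HUD ball counts.
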(event Custom|Remove%20HUD
  ;[1 1 1] Bind Death Event To Remove HUD
  (Widget|RemovefromParent (Variables|Default|GetMyHUD)))

(event Custom|Add%20Default%20Widget
  ;[1 1 1] CUstom Add To Viewport Event
  (bind _returnvalue (UserInterface|CreateWidget "/Game/UI/HUD/WBP_HUD.WBP_HUD_C" (Game|GetPlayerController 0)))
  (bind _output_get (Variables|Default|SetMyHUD _returnvalue))
  (UserInterface|Viewport|AddtoViewport _output_get 0))

(event EventDeathEvent
  ;[1 1 1] Remove HUD when player dies
  ;;[1 1 1] See Above
  (CallFunction|RemoveHUD))

(event EventPossessed
  (params (NewController :type Controller%20Object%20Reference))
  ;[1 1 1] Add HUD To Player Viewport
  (Networking|SwitchHasAuthority
    (:Authority
      (if (Pawn|IsLocallyControlled)
        ;;[1 1 1] See Above
        (CallFunction|AddDefaultWidget)))))

(event EventBeginPlay
  ;[1 1 1] Add HUD To Player Viewport
  (Networking|SwitchHasAuthority
    (:Remote
      (if (Pawn|IsLocallyControlled)
        ;;[1 1 1] See Above
        (CallFunction|AddDefaultWidget)))))

(event Input|KeyboardEvents|1
  (params (Key :type Key%20Structure :default "None"))
  ;[1 1 1] This is Copied From BP_UITestCharacter - Should Not Be Used (Aside From Testing)
  (:Pressed
    (Default|ChangeBallCount (Variables|Default|GetMyHUD) 0 1 true)))

(event Input|KeyboardEvents|2
  (params (Key :type Key%20Structure :default "None"))
  ;[1 1 1] This is Copied From BP_UITestCharacter - Should Not Be Used (Aside From Testing)
  (:Pressed
    (Default|ChangeBallCount (Variables|Default|GetMyHUD) 1 1 true)))

(event Input|KeyboardEvents|3
  (params (Key :type Key%20Structure :default "None"))
  ;[1 1 1] This is Copied From BP_UITestCharacter - Should Not Be Used (Aside From Testing)
  (:Pressed
    (Default|ChangeBallCount (Variables|Default|GetMyHUD) 2 1 true)))

(fn ConstructionScript)