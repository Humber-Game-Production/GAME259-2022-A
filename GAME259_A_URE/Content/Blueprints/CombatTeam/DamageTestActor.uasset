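; DamageTestActor is a test actor that damages the main character on contact.
; When its DamageCollision component begins overlapping a BP_Main_Character, it calls TakeDamage with a fixed amount.
; The trailing Delay feeds nothing, so it does not throttle repeat hits.
; Leftover HealthUpdate bindings and health print debugging are disabled or disconnected, so only the overlap damage runs.
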(event OnComponentBeginOverlap(DamageCollision)
  (params (OverlappedComponent :type Primitive%20Component%20Object%20Reference) (OtherActor :type Actor%20Object%20Reference) (OtherComp :type Primitive%20Component%20Object%20Reference) (OtherBodyIndex :type Integer) (bFromSweep :type Boolean) (SweepResult :type Hit%20Result%20Structure%20%28by%20ref%29))
  (bind _asbp_main_character (Utilities|Casting|CastToBP_Main_Character OtherActor))
  (Class|MainCharacter|TakeDamage _asbp_main_character 1e+01 (Utilities|Struct|MakeDamageEvent))
  (Utilities|FlowControl|Delay 2.0))

(event Custom|HealthUpdate_Event_0
  (params (characterHealth :type Float%20%28single-precision%29))
  ;[1 1 1] Binding delegate event when passing in one parameter
  (Development|PrintString (Utilities|String|Append "Current Health: " (Utilities|String|ToString(Float) characterHealth))))

(event Custom|HealthUpdate_Event_2
  ;[1 1 1] Print Statement when Player is Damaged. Disabled
  ;;[1 1 1] Binding delegate event without variable
)

(event EventBeginPlay
  ;[1 1 1] Print Statement when Player is Damaged. Disabled
)

(event Collision|EventActorBeginOverlap
  (params (OtherActor :type Actor%20Object%20Reference)))

(event EventTick
  (params (DeltaSeconds :type Float%20%28single-precision%29)))

(fn ConstructionScript)